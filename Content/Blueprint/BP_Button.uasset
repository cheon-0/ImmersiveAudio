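; Physical push button with a configurable label that opens the Sub_Test level or triggers quit on BPTurnTable, chosen by ButtonValue.
; VRPawn or third-person character overlap plays a timeline sliding the actor along world X between fixed absolute positions.
; At full travel, if still overlapped, it starts a short level-open timer or calls quit immediately.
; Any end overlap cancels that timer and reverses the slide.
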(event `self.Cube.OnComponentBeginOverlap`
  (params (OverlappedComponent :type "PrimitiveComponent Object Reference") (OtherActor :type "Actor Object Reference") (OtherComp :type "PrimitiveComponent Object Reference") (OtherBodyIndex :type Integer) (bFromSweep :type Boolean) (SweepResult :type "HitResult Structure (by ref)"))
  (bind (_returnvalue_x _returnvalue_y _returnvalue_z) (`KismetMathLibrary.BreakVector` (`self.K2_GetActorLocation`)))
  ;[1 1 1] Legacy
  (set `self.ButtonOverlap` true)
  (`|ExecutionSequence`
    (:`then_0`
      (cast `/Game/VRTemplate/Blueprints/VRPawn` OtherActor)
      (bind (_direction _1s) (`Timeline|Button` :!label _label)
        (:`Update`
          (bind _output_get (set `self.ButtonTransition` _1s))
          (bind _returnvalue (`KismetMathLibrary.Lerp` 380.0 400.0 _output_get))
          (`self.K2_SetActorLocation` (`KismetMathLibrary.MakeVector` _returnvalue _returnvalue_y _returnvalue_z)))
        (:`Finished`
          (if (and (>= _returnvalue 400.0) (`self.ButtonOverlap`))
            (switch `int` (`self.ButtonValue`)
              (:`1`
                ;;[1 1 1] Play : Open sub level
                (bind _returnvalue_2 (`KismetSystemLibrary.K2_SetTimerDelegate` (delegate `EV_OpenSubLevel`) 0.5))
                (set `self.ButtonCancel` _returnvalue_2))
              (:`2`
                ;;[1 1 1] Stop : Quit game
                (`/Game/Blueprint/BP_TurnTableBody.EV_Quit` (`self.BP_TurnTable`))))))))
    (:`then_1`
      (cast `/Game/ThirdPerson/Blueprints/BP_ThirdPersonCharacter` OtherActor)
      (goto _label))))

(event `EV_OpenSubLevel`
  ;[1 1 1] Legacy
  ;;[1 1 1] Play : Open sub level
  (`GameplayStatics.OpenLevelBySoftObjectPtr` "/Game/Level/Sub_Test.Sub_Test"))

(event `self.Cube.OnComponentEndOverlap`
  (params (OverlappedComponent :type "PrimitiveComponent Object Reference") (OtherActor :type "Actor Object Reference") (OtherComp :type "PrimitiveComponent Object Reference") (OtherBodyIndex :type Integer))
  ;[1 1 1] Legacy
  (set `self.ButtonOverlap` false)
  (`KismetSystemLibrary.K2_ClearAndInvalidateTimerHandle` (`self.ButtonCancel`))
  (goto _label :!via `Reverse`))

(fn `UserConstructionScript`
  (`TextRenderComponent.K2_SetText` (`self.TextRender`) (`self.ButtonText`)))